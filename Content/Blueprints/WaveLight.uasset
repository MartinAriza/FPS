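; WaveLight is a light Blueprint that pulses in brightness and changes color when a trigger box is overlapped.
; Tick drives the light's intensity with a sine wave of game time, shaped by Period, Floor and Intensity.
; The trigger box's begin-overlap event sets the point light to the Color value, with no filter on the overlapping actor and no revert.
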(event `self.ReceiveTick`
  (params (DeltaSeconds :type "Float (single-precision)"))
  (`LightComponent.SetIntensity` (`self.LightComponent`) (* (+ (`KismetMathLibrary.Sin` (* (`KismetSystemLibrary.GetGameTimeInSeconds`) (`self.Period`))) (`self.Floor`)) (`self.Intensity`))))

(event `self.TriggerBox.OnActorBeginOverlap`
  (params (OverlappedActor :type "Actor Object Reference") (OtherActor :type "Actor Object Reference"))
  (`LightComponent.SetLightColor` (`self.PointLightComponent`) (`self.Color`) true))

(fn `UserConstructionScript`)