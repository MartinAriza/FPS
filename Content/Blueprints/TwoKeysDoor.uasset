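; TwoKeysDoor is a door actor that a first-person character opens by spending keys on it.
; When hit by a FirstPersonCharacter holding at least one key, it takes one key and decrements its remaining NKeys count.
; The door destroys itself when that count reaches zero, so payment can be spread across several hits.
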(event `self.ReceiveHit`
  (params (MyComp :type "PrimitiveComponent Object Reference") (Other :type "Actor Object Reference") (OtherComp :type "PrimitiveComponent Object Reference") (bSelfMoved :type Boolean) (HitLocation :type "Vector Structure") (HitNormal :type "Vector Structure") (NormalImpulse :type "Vector Structure") (Hit :type "HitResult Structure (by ref)"))
  (bind _nkeys (`self.NKeys`))
  (bind _asfirst_person_character (cast `/Game/Blueprints/FirstPersonCharacter` Other))
  (bind _keys (`/Game/Blueprints/FirstPersonCharacter.Keys` _asfirst_person_character))
  (if (> _keys 0)
    (`/Engine/EditorBlueprintResources/StandardMacros.DecrementInt` _keys
      (:`  `
        (set `self.NKeys` (- _nkeys 1))
        (if (== _nkeys 0)
          (`self.K2_DestroyActor`))))))

(fn `UserConstructionScript`)