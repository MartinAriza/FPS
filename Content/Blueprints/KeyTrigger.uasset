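; KeyTrigger is a key pickup that also opens a door by destroying it.
; It extends a parent class, adding one to the player's Keys count in Taken before calling the parent version.
; On any actor overlap it runs the parent handler, then destroys the referenced Door without checking the overlapping actor or key count.
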(event `self.ReceiveActorBeginOverlap`
  (params (OtherActor :type "Actor Object Reference"))
  (`parent.ReceiveActorBeginOverlap` OtherActor)
  (`self.K2_DestroyActor` (`self.Door`)))

(fn `Taken`
  (params (Player :type "/Game/Blueprints/FirstPersonCharacter Object Reference"))
  (`/Engine/EditorBlueprintResources/StandardMacros.IncrementInt` (`/Game/Blueprints/FirstPersonCharacter.Keys` Player)
    (:`  `
      (`parent.Taken` null))))

(fn `UserConstructionScript`
  (`parent.UserConstructionScript`))